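; Ghost preview actor for RTS building placement that toggles the player controller's building mode.
; ConstructBuilding briefly spawns the building class to read its mesh, name, build time and costs, then starts the preview.
; A gated Tick snaps the preview to the grid at the supplied cursor position and swaps its material on overlaps, ignoring fog-blocking volumes.
; SetConstructionStructure packages the building data and transform into a construction struct.
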(event `SpawnPreview`
  (params (`Building Class` :type "/Game/RTS_Test/Blueprints/Buildings/RTS_BuildingMaster_BP Class Reference") (DisplayMesh :type "StaticMesh Object Reference") (ConstuctionTime :type "Float (double-precision)") (BuildingName :type "/Game/RTS_Test/Blueprints/Enums/BuildingName_ENUM Enum" :default "NewEnumerator0") (WoodCost :type Integer) (OreCost :type Integer))
  (if (`self.IsPreviewing`)
    (`self.DestroyPreview`))
  (`self.SetBuildingDetails` `Building Class` DisplayMesh ConstuctionTime BuildingName WoodCost OreCost)
  (bind _output_get (set `self.IsPreviewing` true))
  (`/Game/RTS_Test/Blueprints/GameSettings/RTS_PlayerController_BP.SetBuildingModeActive` (`self.PlayerControllerRef`) _output_get)
  (`StaticMeshComponent.SetStaticMesh` (`self.PreviewBuildingMesh`) (`self.DisplayMesh`))
  (`self.OpenGate`))

(event `DestroyPreview`
  (`self.CloseGate`)
  (set `self.BuildingClass` null)
  (set `self.DisplayMesh` null)
  (bind _output_get (set `self.IsPreviewing` false))
  (`/Game/RTS_Test/Blueprints/GameSettings/RTS_PlayerController_BP.SetBuildingModeActive` (`self.PlayerControllerRef`) _output_get)
  (`StaticMeshComponent.SetStaticMesh` (`self.PreviewBuildingMesh`) (`self.DisplayMesh`))
  (`self.K2_SetActorRotation` (struct)))

(event `/Game/RTS_Test/Blueprints/Library/RTS_Constuction_IF.ConstructBuilding`
  (params (BuildingMasterClass :type "/Game/RTS_Test/Blueprints/Buildings/RTS_BuildingMaster_BP Class Reference"))
  (bind _returnvalue (`|SpawnActorFromClass` BuildingMasterClass (`self.EmprtTransform`) "AlwaysSpawn" "OverrideRootScale" null null true "NewEnumerator0" null))
  (`|ExecutionSequence`
    (:`then_0`
      (bind _asrts_building_master_bp (castclass `/Game/RTS_Test/Blueprints/Buildings/RTS_BuildingMaster_BP` BuildingMasterClass))
      (`self.DestroyPreview`)
      (`self.SpawnPreview` _asrts_building_master_bp (`/Game/RTS_Test/Blueprints/Buildings/RTS_BuildingMaster_BP.DisplayMesh` _returnvalue) (`/Game/RTS_Test/Blueprints/Buildings/RTS_BuildingMaster_BP.ConstructionTime` _returnvalue) (`/Game/RTS_Test/Blueprints/Buildings/RTS_BuildingMaster_BP.BuildingName` _returnvalue) (`/Game/RTS_Test/Blueprints/Buildings/RTS_BuildingMaster_BP.WoodCost` _returnvalue) (`/Game/RTS_Test/Blueprints/Buildings/RTS_BuildingMaster_BP.OreCost` _returnvalue)))
    (:`then_1`
      (`self.K2_DestroyActor` _returnvalue))))

(event `self.ReceiveTick`
  (params (DeltaSeconds :type "Float (single-precision)"))
  (bind _previewbuildingmesh (`self.PreviewBuildingMesh`))
  (`/Engine/EditorBlueprintResources/StandardMacros.Gate` true :!label _label
    (:`Exit`
      (`self.K2_SetActorLocation` self (`self.GridSnap`) false false)
      (if (`self.CheckOverlap`)
        (`PrimitiveComponent.SetMaterial` _previewbuildingmesh 0 "/Game/RTS_Test/Materials/Structures/PreviewBad_Mat_Inst.PreviewBad_Mat_Inst")
        (else
          (`PrimitiveComponent.SetMaterial` _previewbuildingmesh 0 "/Game/RTS_Test/Materials/Structures/Preview_Mat_Inst.Preview_Mat_Inst"))))))

(event `OpenGate`
  (goto _label :!via `Open`))

(event `CloseGate`
  (goto _label :!via `Close`))

(fn `CheckOverlap`
  (returns (IsOverlapping :type Boolean))
  (bind _previewbuildingmesh (`self.PreviewBuildingMesh`))
  (return (> (- (`KismetArrayLibrary.Array_Length` (`PrimitiveComponent.GetOverlappingActors` _previewbuildingmesh null)) (`KismetArrayLibrary.Array_Length` (`PrimitiveComponent.GetOverlappingActors` _previewbuildingmesh "/Script/VaFogOfWar.VaFogBlockingVolume"))) 0)))

(fn `GridSnap`
  (returns (SnapPosition :type "Vector Structure"))
  (bind (_mouseinworldpos_x _mouseinworldpos_y _mouseinworldpos_z) (`KismetMathLibrary.BreakVector` (`self.MouseInWorldPos`)))
  (bind _snapvalue (`self.SnapValue`))
  (bind _snapvalue_2 (`self.SnapValue`))
  (return (`KismetMathLibrary.MakeVector` (`KismetMathLibrary.Conv_IntToDouble` (* (/ (`KismetMathLibrary.FFloor` (+ _mouseinworldpos_x 50.0)) _snapvalue) _snapvalue)) (`KismetMathLibrary.Conv_IntToDouble` (* (/ (`KismetMathLibrary.FFloor` (+ _mouseinworldpos_y 50.0)) _snapvalue_2) _snapvalue_2)) _mouseinworldpos_z)))

(fn `SetBuildingDetails`
  (params (BuildingClass :type "/Game/RTS_Test/Blueprints/Buildings/RTS_BuildingMaster_BP Class Reference") (DisplayMesh :type "StaticMesh Object Reference") (ConstuctionTime :type "Float (double-precision)") (BuildingName :type "/Game/RTS_Test/Blueprints/Enums/BuildingName_ENUM Enum" :default "NewEnumerator0") (WoodCost :type Integer) (OreCost :type Integer))
  (set `self.BuildingClass` BuildingClass)
  (set `self.DisplayMesh` DisplayMesh)
  (set `self.ConstuctionTime` ConstuctionTime)
  (set `self.BuildingName` BuildingName)
  (set `self.WoodCost` WoodCost)
  (set `self.OreCost` OreCost))

(fn `SetConstructionStructure`
  (returns (ConstructionStruct :type "/Game/RTS_Test/Blueprints/Structures/RTS_Construction_Struct Structure"))
  (set `self.ConstructionStructure` (make `/Game/RTS_Test/Blueprints/Structures/RTS_Construction_Struct` false (`self.BuildingClass`) (`self.GetTransform`) (`self.DisplayMesh`) (`self.BuildingName`) (`self.ConstuctionTime`)))
  (return (`self.ConstructionStructure`)))

(fn `SetCursorPosition`
  (params (CursorPosition :type "Vector Structure"))
  (set `self.MouseInWorldPos` CursorPosition)
  (return))

(fn `UserConstructionScript`)
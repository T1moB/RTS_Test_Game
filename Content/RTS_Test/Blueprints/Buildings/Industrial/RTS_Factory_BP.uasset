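; RTS factory building that refines wood and ore into metal and manufactures ground vehicles paid for with that metal.
; A looping timer produces metal until inputs run short or storage fills, then warns on the HUD and stops.
; Vehicle orders join a queue mirrored to the building HUD, with refunds on cancellation.
; A second looping timer spawns each vehicle at an X offset from the factory, clearing once a spawn empties the queue.
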(event `self.StartResourceProduction`
  (set `self.IsProducingResource` true)
  (`Button.SetColorAndOpacity` (`/Game/RTS_Test/Blueprints/Widgets/BuildingInfo_HUD.ProduceResourceBTN` (`self.BuildingHudRef`)) (struct :`R` 0.25 :`G` 0.25 :`B` 0.25 :`A` 1.0))
  (bind _returnvalue (`KismetSystemLibrary.K2_SetTimer` null "ProduceRefinedMetal" 10.0 true))
  (set `self.ProduceResourceTimer` _returnvalue))

(event `self.StopResourceProduction`
  (set `self.IsProducingResource` false)
  (`Button.SetColorAndOpacity` (`/Game/RTS_Test/Blueprints/Widgets/BuildingInfo_HUD.ProduceResourceBTN` (`self.BuildingHudRef`)) (struct :`R` 1.0 :`G` 1.0 :`B` 1.0 :`A` 1.0))
  (bind _output_get (set `self.ProduceResourceTimer` (struct)))
  (`KismetSystemLibrary.K2_ClearAndInvalidateTimerHandle` _output_get))

(event `self.ManufactureVehicle`
  (bind _playercontrollerref (`self.PlayerControllerRef`))
  (if (>= (`/Game/RTS_Test/Blueprints/GameSettings/RTS_PlayerController_BP.RefinedMetalResource` _playercontrollerref) (`self.VehicleCost`))
    (set `/Game/RTS_Test/Blueprints/GameSettings/RTS_PlayerController_BP.RefinedMetalResource` (- (`/Game/RTS_Test/Blueprints/GameSettings/RTS_PlayerController_BP.RefinedMetalResource` _playercontrollerref) (`self.VehicleCost`)) _playercontrollerref)
    (bind _result (`/Engine/EditorBlueprintResources/StandardMacros.IncrementInt` (`self.AmountToManufacture`))
      (:`  `
        (bind _output_get (set `self.AmountToManufacture` _result))
        (`self.UpdateVehicleQueue`)
        (if (== _output_get 1)
          (bind _returnvalue (`KismetSystemLibrary.K2_SetTimer` null "SpawnVehicle" 20.0 true))
          (set `self.VehicleSpawnTimer` _returnvalue))))
    (else
      (`/Game/RTS_Test/Blueprints/Widgets/MainGameUI_HUD.TriggerText` (`/Game/RTS_Test/Blueprints/GameSettings/RTS_PlayerController_BP.MainGameHudRef` _playercontrollerref)))))

(event `self.DecreaseVehicleQueue`
  (params (`Index Ref` :type Integer))
  (bind _playercontrollerref (`self.PlayerControllerRef`))
  (set `/Game/RTS_Test/Blueprints/GameSettings/RTS_PlayerController_BP.RefinedMetalResource` (+ (`/Game/RTS_Test/Blueprints/GameSettings/RTS_PlayerController_BP.RefinedMetalResource` _playercontrollerref) (`self.VehicleCost`)) _playercontrollerref)
  (bind _result (`/Engine/EditorBlueprintResources/StandardMacros.DecrementInt` (`self.AmountToManufacture`))
    (:`  `
      (set `self.AmountToManufacture` _result)
      (`self.RemoveVehicleFromQueue` `Index Ref`))))

(fn `GetManufactureQueueLenght`
  (returns (QueueCount :type Integer))
  (return (`KismetArrayLibrary.Array_Length` (`self.VehiclesToManufacture`))))

(fn `GetSpawnTransform`
  (returns (Transform :type "Transform Structure"))
  (bind (_returnvalue_x _returnvalue_y _returnvalue_z) (`KismetMathLibrary.BreakVector` (`self.K2_GetActorLocation` self)))
  (bind (_returnvalue_roll _returnvalue_pitch _returnvalue_yaw) (`KismetMathLibrary.BreakRotator` (`self.K2_GetActorRotation` self)))
  (return (`KismetMathLibrary.MakeTransform` (`KismetMathLibrary.MakeVector` (+ _returnvalue_x 1500.0) _returnvalue_y (+ _returnvalue_z 50.0)) (`KismetMathLibrary.MakeRotator` _returnvalue_roll _returnvalue_pitch _returnvalue_yaw))))

(fn `ProduceRefinedMetal`
  (locals (OreCostLocal :type "Float (double-precision)") (WoodCostLocal :type "Float (double-precision)"))
  (bind _playercontrollerref (`self.PlayerControllerRef`))
  (bind _playercontrollerref_2 (`self.PlayerControllerRef`))
  (bind _playercontrollerref_3 (`self.PlayerControllerRef`))
  (bind _maingamehudref (`/Game/RTS_Test/Blueprints/GameSettings/RTS_PlayerController_BP.MainGameHudRef` (`self.PlayerControllerRef`)))
  (if (and (>= (`/Game/RTS_Test/Blueprints/GameSettings/RTS_PlayerController_BP.WoodResources` _playercontrollerref) (`local.WoodCostLocal`)) (>= (`/Game/RTS_Test/Blueprints/GameSettings/RTS_PlayerController_BP.OreResources` _playercontrollerref) (`local.OreCostLocal`)))
    (if (<= (+ (`/Game/RTS_Test/Blueprints/GameSettings/RTS_PlayerController_BP.RefinedMetalResource` _playercontrollerref_2) 1.0) (`/Game/RTS_Test/Blueprints/GameSettings/RTS_PlayerController_BP.MaxRefinedMetalResource` _playercontrollerref_2))
      (set `/Game/RTS_Test/Blueprints/GameSettings/RTS_PlayerController_BP.WoodResources` (- (`/Game/RTS_Test/Blueprints/GameSettings/RTS_PlayerController_BP.WoodResources` _playercontrollerref_3) (`local.WoodCostLocal`)) _playercontrollerref_3)
      (set `/Game/RTS_Test/Blueprints/GameSettings/RTS_PlayerController_BP.OreResources` (- (`/Game/RTS_Test/Blueprints/GameSettings/RTS_PlayerController_BP.OreResources` _playercontrollerref_3) (`local.OreCostLocal`)) _playercontrollerref_3)
      (set `/Game/RTS_Test/Blueprints/GameSettings/RTS_PlayerController_BP.RefinedMetalResource` (+ (`/Game/RTS_Test/Blueprints/GameSettings/RTS_PlayerController_BP.RefinedMetalResource` _playercontrollerref_3) 1.0) _playercontrollerref_3)
      (return)
      (else
        (`/Game/RTS_Test/Blueprints/Widgets/MainGameUI_HUD.TriggerStorageText` _maingamehudref)
        (`self.StopResourceProduction`)
        (return)))
    (else
      (`/Game/RTS_Test/Blueprints/Widgets/MainGameUI_HUD.TriggerText` _maingamehudref)
      (`self.StopResourceProduction`)
      (return))))

(fn `RemoveVehicleFromQueue`
  (params (Index :type Integer))
  (`KismetArrayLibrary.Array_Remove` (`self.VehiclesToManufacture`) Index)
  (message `/Game/RTS_Test/Blueprints/Library/RTS_OccupantInfo_IF.SetVehicleQueue` (`self.BuildingHudRef`) (`self.VehiclesToManufacture`))
  (`/Game/RTS_Test/Blueprints/Widgets/BuildingInfo_HUD.UpdateManufactureQueue` (`self.BuildingHudRef`))
  (return))

(fn `SpawnVehicle`
  (bind _returnvalue (`|SpawnActorFromClass` "/Game/RTS_Test/Blueprints/Units/GroundVehicles/RTS_GroundVehicleMaster.RTS_GroundVehicleMaster_C" (`self.GetSpawnTransform`) "Undefined" "OverrideRootScale" null "NewEnumerator1" null))
  (`/Game/RTS_Test/Blueprints/Units/GroundVehicles/RTS_GroundVehicleMaster.OnManufacture` _returnvalue)
  (bind _result (`/Engine/EditorBlueprintResources/StandardMacros.DecrementInt` (`self.AmountToManufacture`))
    (:`  `
      (set `self.AmountToManufacture` _result)
      (`self.RemoveVehicleFromQueue` 0)
      (if (not (> (`self.AmountToManufacture`) 0))
        (`KismetSystemLibrary.K2_ClearAndInvalidateTimerHandle` (`self.VehicleSpawnTimer`)))
      (return))))

(fn `UpdateVehicleQueue`
  (`KismetArrayLibrary.Array_Add` (`self.VehiclesToManufacture`) (`self.Vehicle`))
  (message `/Game/RTS_Test/Blueprints/Library/RTS_OccupantInfo_IF.SetVehicleQueue` (`self.BuildingHudRef`) (`self.VehiclesToManufacture`))
  (`/Game/RTS_Test/Blueprints/Widgets/BuildingInfo_HUD.UpdateManufactureQueue` (`self.BuildingHudRef`))
  (return))

(fn `UserConstructionScript`
  (`parent.UserConstructionScript`))
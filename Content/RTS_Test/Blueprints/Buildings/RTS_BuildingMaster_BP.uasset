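; Base building actor for an RTS that units can enter to construct, with its own info HUD.
; An entry box sized from the mesh bounds notifies units targeting it when they arrive, and an occupant list feeds the HUD.
; While occupied and under construction, Tick advances a clock using game speed divided by occupant count.
; On completion it releases occupants and swaps the preview material for the wall material.
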(event `self.ReceiveBeginPlay`
  (`|ExecutionSequence`
    (:`then_0`
      (`self.ReferenceCast`))
    (:`then_1`
      (add `/Game/RTS_Test/Blueprints/GameSettings/RTS_GameStateBase_BP.GameSpeedControl` (`self.GameStateRef`) (`|CreateDelegate` :!event `GetGameSpeed`))
      (bind _gamespeed (`/Game/RTS_Test/Blueprints/GameSettings/RTS_GameStateBase_BP.GetGameSpeed` (`self.GameStateRef`)))
      (set `self.GameSpeed` _gamespeed))
    (:`then_2`
      (add `/Game/RTS_Test/Blueprints/GameSettings/RTS_PlayerController_BP.DisplayHud` (`self.PlayerControllerRef`) (`|CreateDelegate` :!event `DisplayBuildingHud`)))))

(event `OnSpawn`
  (set `self.IsUnderConstruction` true))

(event `GetGameSpeed`
  (params (GameSpeed :type "Float (double-precision)"))
  (set `self.GameSpeed` GameSpeed))

(event `self.ReceiveTick`
  (params (DeltaSeconds :type "Float (single-precision)"))
  (set `self.DeltaTime` DeltaSeconds)
  (if (`self.CheckConstructionStatus`)
    (`self.ConstructBuilding`)
    (if (>= (`self.TimeWorked`) (`self.ConstructionTime`))
      (set `self.IsBuilt` true)
      (set `self.IsUnderConstruction` false)
      (`self.ReleaseAllOccupants`)
      (`self.ClearOccupantList`)
      (`PrimitiveComponent.SetMaterial` (`self.BuildingMesh`) 0 "/Game/StarterContent/Materials/M_Basic_Wall.M_Basic_Wall"))))

(event `DisplayBuildingHud`
  (params (Actor :type "Actor Object Reference") (Bypass :type Boolean))
  (bind _playercontrollerref (`self.PlayerControllerRef`))
  (if (== Actor self)
    (`UserWidget.AddToViewport` (`self.BuildingHudRef`) 1)
    (`WidgetBlueprintLibrary.SetInputMode_UIOnlyEx` _playercontrollerref null)
    (`Widget.SetIsEnabled` (`/Game/RTS_Test/Blueprints/GameSettings/RTS_PlayerController_BP.MainGameHudRef` _playercontrollerref) true)))

(event `self.EntryPoint.OnComponentBeginOverlap`
  (params (OverlappedComponent :type "PrimitiveComponent Object Reference") (OtherActor :type "Actor Object Reference") (OtherComp :type "PrimitiveComponent Object Reference") (OtherBodyIndex :type Integer) (bFromSweep :type Boolean) (SweepResult :type "HitResult Structure (by ref)"))
  (bind _asrts_ground_unit_master (cast `/Game/RTS_Test/Blueprints/Units/RTS_GroundUnitMaster` OtherActor))
  (set `self.SelectedUnit` _asrts_ground_unit_master)
  (if (== (`/Game/RTS_Test/Blueprints/Units/RTS_GroundUnitMaster.TargetBuilding` (`self.SelectedUnit`)) self)
    (`/Game/RTS_Test/Blueprints/Units/RTS_GroundUnitMaster.ArriveAtBuilding` (`self.SelectedUnit`))))

(fn `CheckConstructionStatus`
  (returns (ReturnValue :type Boolean))
  (return (and (`self.IsUnderConstruction`) (not (`self.IsBuilt`)) (> (`KismetArrayLibrary.Array_Length` (`self.Occupants`)) 0))))

(fn `ClearOccupantList`
  (bind _buildinghudref (`self.BuildingHudRef`))
  (`KismetArrayLibrary.Array_Clear` (`self.Occupants`))
  (message `/Game/RTS_Test/Blueprints/Library/RTS_OccupantInfo_IF.SetOccupantNames` _buildinghudref (`self.Occupants`))
  (`/Game/RTS_Test/Blueprints/Widgets/BuildingInfo_HUD.UpdateOccupantList` _buildinghudref)
  (return))

(fn `ConstructBuilding`
  (bind _output_get (set `self.GameClock` (`/Game/RTS_Test/Blueprints/Library/FuncLib.SetGameTime` (`self.DeltaTime`) (/ (`self.GameSpeed`) (`KismetMathLibrary.Conv_IntToDouble` (`KismetArrayLibrary.Array_Length` (`self.Occupants`)))) (`self.GameClock`))))
  (set `self.TimeWorked` (* _output_get (`self.ConstructionModifier`) 60.0)))

(fn `ReleaseAllOccupants`
  (for _array_element (`self.Occupants`)
    (`/Game/RTS_Test/Blueprints/Units/RTS_GroundUnitMaster.SetTargetable` _array_element))
  (`KismetArrayLibrary.Array_Clear` (`self.Occupants`))
  (return))

(fn `ReleaseSingleOccupant`
  (params (TargetUnit :type "/Game/RTS_Test/Blueprints/Units/RTS_GroundUnitMaster Object Reference"))
  (bind _occupants (`self.Occupants`))
  (bind _buildinghudref (`self.BuildingHudRef`))
  (`/Game/RTS_Test/Blueprints/Units/RTS_GroundUnitMaster.SetTargetable` TargetUnit)
  (for (_array_element _array_index) _occupants
    (if (== _array_element TargetUnit)
      (`KismetArrayLibrary.Array_Remove` _occupants _array_index)
      (message `/Game/RTS_Test/Blueprints/Library/RTS_OccupantInfo_IF.SetOccupantNames` _buildinghudref (`self.Occupants`))
      (`/Game/RTS_Test/Blueprints/Widgets/BuildingInfo_HUD.UpdateOccupantList` _buildinghudref)
      (return))))

(fn `SetConstructionTime`
  (params (ConstructionTimeRaw :type "Float (double-precision)"))
  (set `self.ConstructionTime` (* ConstructionTimeRaw 60.0))
  (return))

(fn `SetOccupantNames`
  (params (Units :type "Array of /Game/RTS_Test/Blueprints/Units/RTS_GroundUnitMaster Object Reference (by ref)"))
  (returns (Succes :type Boolean))
  (return false))

(fn `SetUnit`
  (params (TargetUnit :type "/Game/RTS_Test/Blueprints/Units/RTS_GroundUnitMaster Object Reference"))
  (`KismetArrayLibrary.Array_AddUnique` (`self.Occupants`) TargetUnit)
  (message `/Game/RTS_Test/Blueprints/Library/RTS_OccupantInfo_IF.SetOccupantNames` (`self.BuildingHudRef`) (`self.Occupants`))
  (`/Game/RTS_Test/Blueprints/Widgets/BuildingInfo_HUD.UpdateOccupantList` (`self.BuildingHudRef`))
  (return))

(fn `UserConstructionScript`
  (`StaticMeshComponent.SetStaticMesh` (`self.BuildingMesh`) (`self.DisplayMesh`))
  (`BoxComponent.SetBoxExtent` (`self.EntryPoint`) (`.Max` (`StaticMeshComponent.GetLocalBounds` (`self.BuildingMesh`))) true)
  (if (`self.IsBuilt`)
    (`PrimitiveComponent.SetMaterial` (`self.BuildingMesh`) 0 "/Game/StarterContent/Materials/M_Basic_Wall.M_Basic_Wall")
    (else
      (`PrimitiveComponent.SetMaterial` (`self.BuildingMesh`) 0 "/Game/RTS_Test/Materials/Structures/Preview_Mat_Inst.Preview_Mat_Inst"))))
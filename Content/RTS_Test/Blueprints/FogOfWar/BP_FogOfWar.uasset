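; Fog of war Blueprint that blurs the BlackFog upscale texture into RT_Result every Tick.
; It uses a multi-pass Kawase blur: one M_Kawase dynamic material alternates between ping and pong render targets, with the Shift offset growing each pass.
; KawaseSteps sets the pass count, and the last pass writes to RT_Result.
; The construction script also creates an M_SubtractionOfFog material instance but does not store it.
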(event `self.ReceiveBeginPlay`
  (bind _returnvalue (`KismetMaterialLibrary.CreateDynamicMaterialInstance` "/Game/RTS_Test/Materials/Blur/M_Kawase.M_Kawase"))
  (bind _output_get (set `self.Kawase Pass` _returnvalue))
  (`MaterialInstanceDynamic.SetScalarParameterValue` _output_get "Resolution" (`KismetMathLibrary.Conv_IntToDouble` (`self.Input Resolution X`))))

(event `self.ReceiveTick`
  (params (DeltaSeconds :type "Float (single-precision)"))
  (bind _kawase_pass (`self.Kawase Pass`))
  (bind _kawase_pass_2 (`self.Kawase Pass`))
  (`|ExecutionSequence`
    (:`then_0`
      (`MaterialInstanceDynamic.SetTextureParameterValue` _kawase_pass "Texture" (`VaFogLayer.UpscaleTexture` (`self.BlackFog`)))
      (`MaterialInstanceDynamic.SetScalarParameterValue` _kawase_pass "Shift" 0.0)
      (`KismetRenderingLibrary.DrawMaterialToRenderTarget` (select `bool` (== (`self.Kawase Steps`) 1) :`false` "/Game/RTS_Test/Materials/Blur/RT_Kawase_Ping.RT_Kawase_Ping" :`true` "/Game/RTS_Test/Materials/Blur/RT_Result.RT_Result" :!type "TextureRenderTarget2D Object Reference") _kawase_pass))
    (:`then_1`
      (for _index (range 2 (+ (`self.Kawase Steps`) 1))
        (`MaterialInstanceDynamic.SetScalarParameterValue` (`self.Kawase Pass`) "Shift" (- (`KismetMathLibrary.Conv_IntToDouble` _index) 0.5))
        (bind _returnvalue (mod _index 2))
        (`MaterialInstanceDynamic.SetTextureParameterValue` _kawase_pass_2 "Texture" (select `bool` (!= _returnvalue 0) :`false` "/Game/RTS_Test/Materials/Blur/RT_Kawase_Ping.RT_Kawase_Ping" :`true` "/Game/RTS_Test/Materials/Blur/RT_Kawase_Pong.RT_Kawase_Pong" :!type "TextureRenderTarget2D Object Reference"))
        (`KismetRenderingLibrary.DrawMaterialToRenderTarget` (select `bool` (== _index (`self.Kawase Steps`)) :`false` (select `bool` (== _returnvalue 0) :`false` "/Game/RTS_Test/Materials/Blur/RT_Kawase_Ping.RT_Kawase_Ping" :`true` "/Game/RTS_Test/Materials/Blur/RT_Kawase_Pong.RT_Kawase_Pong" :!type "TextureRenderTarget2D Object Reference") :`true` "/Game/RTS_Test/Materials/Blur/RT_Result.RT_Result") _kawase_pass_2)))))

(fn `UserConstructionScript`
  (`KismetMaterialLibrary.CreateDynamicMaterialInstance` "/Game/RTS_Test/Materials/Fog/M_SubtractionOfFog.M_SubtractionOfFog"))
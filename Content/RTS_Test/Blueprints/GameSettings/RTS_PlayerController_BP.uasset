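; RTS player controller that drives the camera pawn, unit selection and orders, and building placement.
; BeginPlay caches camera, game state and marquee HUD, then spawns the construction preview, construction manager and main HUD.
; Primary click places buildings or drives marquee selection; secondary cancels placement, shows unit HUD, or moves selected units and vehicles, boarding units into targeted vehicles.
; Camera supports edge scroll, axis movement, pan, zoom and boost; B and V debug-spawn vehicles and units.
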(event `InputAction|RotatePreviewRight`
  (params (Key :type "Key Structure"))
  (bind _constructionpreviewref (`self.ConstructionPreviewRef`))
  (bind (_returnvalue_roll _returnvalue_pitch _returnvalue_yaw) (`KismetMathLibrary.BreakRotator` (`self.K2_GetActorRotation` _constructionpreviewref)))
  (:`Pressed`
    (set `self.DisableCameraMovement` true)
    (if (and (`self.IsBuildingModeActive`) (!= _constructionpreviewref null))
      (`self.K2_SetActorRotation` _constructionpreviewref (`KismetMathLibrary.MakeRotator` _returnvalue_roll _returnvalue_pitch (+ _returnvalue_yaw (`self.ConstructionRotationRate`))) false)))
  (:`Released`
    (set `self.DisableCameraMovement` false)))

(event `self.ReceiveBeginPlay`
  (`|ExecutionSequence`
    (:`then_0`
      (`self.ReferenceCast`) ; Should always be first
    )
    (:`then_1`
      (bind _returnvalue (`|SpawnActorFromClass` "/Game/RTS_Test/Blueprints/Buildings/RTS_PreviewBuilding_BP.RTS_PreviewBuilding_BP_C" (`self.EmptyTransform`) "AlwaysSpawn" "OverrideRootScale" null self null))
      (set `self.ConstructionPreviewRef` _returnvalue)
      (bind _returnvalue_2 (`|SpawnActorFromClass` "/Game/RTS_Test/Blueprints/Buildings/RTS_ConstructionManager_BP.RTS_ConstructionManager_BP_C" (`self.EmptyTransform`) "AlwaysSpawn" "OverrideRootScale" null self null))
      (set `self.ConstructionManagerRef` _returnvalue_2))
    (:`then_2`
      (`self.SpawnWidgets`)
      (`UserWidget.AddToViewport` (`self.MainGameHudRef`) 1)
      (`self.SetHudVisibility` "Visible"))
    (:`then_3`
      (`WidgetBlueprintLibrary.SetInputMode_GameAndUIEx` self null "DoNotLock" false))))

(event `InputAction|RotatePreviewLeft`
  (params (Key :type "Key Structure"))
  (bind _constructionpreviewref (`self.ConstructionPreviewRef`))
  (bind (_returnvalue_roll _returnvalue_pitch _returnvalue_yaw) (`KismetMathLibrary.BreakRotator` (`self.K2_GetActorRotation` _constructionpreviewref)))
  (:`Pressed`
    (set `self.DisableCameraMovement` true)
    (if (and (`self.IsBuildingModeActive`) (!= _constructionpreviewref null))
      (`self.K2_SetActorRotation` _constructionpreviewref (`KismetMathLibrary.MakeRotator` _returnvalue_roll _returnvalue_pitch (- _returnvalue_yaw (`self.ConstructionRotationRate`))) false)))
  (:`Released`
    (set `self.DisableCameraMovement` false)))

(event `self.ReceiveTick`
  (params (DeltaSeconds :type "Float (single-precision)"))
  (set `self.DeltaTime` DeltaSeconds)
  (if (`self.IsHoldingInput`)
    (`self.UpdateMarquee`)
    (elif (and (`self.IsBuildingModeActive`) (!= (`self.ConstructionPreviewRef`) null))
      (`/Game/RTS_Test/Blueprints/Buildings/RTS_PreviewBuilding_BP.SetCursorPosition` (`self.ConstructionPreviewRef`) (`/Game/RTS_Test/Blueprints/Library/FuncLib.GetMousePosInWorld` self 10000.0)))))

(event `InputAxisKey|MouseX`
  (params (AxisValue :type "Float (single-precision)"))
  ;[1 1 1] Edge scroll movement
  (if (not (`self.DisableCameraMovement`))
    (bind (_deltaspeedx _deltaspeedy) (`self.EdgeScroll` :!label _label))
    (`self.CameraMovement` _deltaspeedx _deltaspeedy)))

(event `InputAction|Pan`
  (params (Key :type "Key Structure"))
  (bind _camerapawnref (`self.CameraPawnRef`))
  ;[1 1 1] Camera panning
  ;;[1 1 1] Camera turning
  (:`Pressed`
    (set `self.DisableCameraMovement` true)
    (goto _label_2 :!via `Open`))
  (:`Released`
    (set `self.DisableCameraMovement` false)
    (goto _label_2 :!via `Close`)))

(event `InputAxis|ZoomIn`
  (params (AxisValue :type "Float (single-precision)"))
  (bind _springarm (`/Game/RTS_Test/Blueprints/GameSettings/CameraPawn_BP.SpringArm` (`self.CameraPawnRef`)))
  ;[1 1 1] Camera Zoom
  ;;[1 1 1] Zoom in and out
  (set `SpringArmComponent.TargetArmLength` (`KismetMathLibrary.FClamp` (+ (`SpringArmComponent.TargetArmLength` _springarm) (* AxisValue (`self.ZoomSpeed`))) (`self.MinZoomLimit`) (`self.MaxZoomLimit`)) _springarm))

(event `InputAxisKey|MouseY`
  (params (AxisValue :type "Float (single-precision)"))
  ;[1 1 1] Edge scroll movement
  (if (not (`self.DisableCameraMovement`))
    (goto _label :!via `MouseY`)))

(event `InputAxisKey|MouseX`
  (params (AxisValue :type "Float (single-precision)"))
  (bind _camerapawnref (`self.CameraPawnRef`))
  ;[1 1 1] Camera panning
  ;;[1 1 1] Camera turning
  (`/Engine/EditorBlueprintResources/StandardMacros.Gate` true :!label _label_2
    (:`Exit`
      (`self.K2_SetActorRotation` _camerapawnref (`KismetMathLibrary.MakeRotator` (.roll (`self.K2_GetActorRotation` _camerapawnref)) (.pitch (`self.K2_GetActorRotation` _camerapawnref)) (+ (.yaw (`self.K2_GetActorRotation` _camerapawnref)) (* AxisValue (`self.PanSpeed`)))) false))))

(event `UpdateMarquee`
  (if (`self.IsHoldingInput`)
    (set `self.HoldingTime` (+ (`self.HoldingTime`) (`self.DeltaTime`)))
    (message `/Game/RTS_Test/Blueprints/Library/MarqueeSelection_IF.OnInputHold` (`self.MarqueeHudRef`))))

(event `InputAction|ZoomReset`
  (params (Key :type "Key Structure"))
  ;[1 1 1] Camera Zoom
  ;;[1 1 1] Zoom Reset
  (:`Pressed`
    (set `SpringArmComponent.TargetArmLength` (`self.StartZoom`) (`/Game/RTS_Test/Blueprints/GameSettings/CameraPawn_BP.SpringArm` (`self.CameraPawnRef`)))))

(event `InputAxis|MoveForward`
  (params (AxisValue :type "Float (single-precision)"))
  ;[1 1 1] Camera Movement
  (if (not (`self.DisableCameraMovement`)) :!label _label_3
    (`self.CameraMovement` AxisValue (stale `InputAxis|MoveRight` AxisValue))))

(event `InputAction|Pan`
  (params (Key :type "Key Structure"))
  (bind _camerapawnref (`self.CameraPawnRef`))
  ;[1 1 1] Camera panning
  ;;[1 1 1] Camera turning
  (:`Pressed`
    (goto _label_4 :!via `Open`))
  (:`Released`
    (goto _label_4 :!via `Close`)))

(event `InputAxis|MoveRight`
  (params (AxisValue :type "Float (single-precision)"))
  ;[1 1 1] Camera Movement
  (goto _label_3))

(event `InputAxisKey|MouseY`
  (params (AxisValue :type "Float (single-precision)"))
  (bind _camerapawnref (`self.CameraPawnRef`))
  ;[1 1 1] Camera panning
  ;;[1 1 1] Camera turning
  (`/Engine/EditorBlueprintResources/StandardMacros.Gate` true :!label _label_4
    (:`Exit`
      (`self.K2_SetActorRotation` _camerapawnref (`KismetMathLibrary.MakeRotator` (.roll (`self.K2_GetActorRotation` _camerapawnref)) (`KismetMathLibrary.FClamp` (+ (.pitch (`self.K2_GetActorRotation` _camerapawnref)) (* AxisValue (`self.PanSpeed`))) -25.0 50.0) (.yaw (`self.K2_GetActorRotation` _camerapawnref))) false))))

(event `InputAction|FastCamera`
  (params (Key :type "Key Structure"))
  ;[1 1 1] Set Camera Boost
  (:`Pressed`
    (set `self.MovementSpeedModifier` 2.0))
  (:`Released`
    (set `self.MovementSpeedModifier` 1.0)))

(event `InputAction|SecondaryAction`
  (params (Key :type "Key Structure"))
  (bind (_hitresult _returnvalue) (`self.GetHitResultUnderCursorByChannel` "TraceTypeQuery1" false))
  (bind (_bblockinghit _binitialoverlap _time _distance _location _impactpoint _normal _impactnormal _physmat _hitactor) (`GameplayStatics.BreakHitResult` _hitresult))
  (:`Pressed`
    (if (`self.IsBuildingModeActive`)
      (`/Game/RTS_Test/Blueprints/Buildings/RTS_PreviewBuilding_BP.DestroyPreview` (`self.ConstructionPreviewRef`))
      (elif (`self.IsUnitSelected`)
        (if _returnvalue
          (set `self.TargetLocation` _location)
          (set `self.HitActor` _hitactor)
          (`|ExecutionSequence`
            (:`then_0`
              (`self.UnitMovement`
                (:`MoveToLocation`
                  (`self.RemoveLocationDecal`))
                (:`MoveToVehicle`
                  (`self.GetInVehicle`))))
            (:`then_1`
              (`self.VehicleMovement`))))
        (else
          (`self.GetUnitHud`))))))

(event `InputAction|PanReset`
  (params (Key :type "Key Structure"))
  (bind _camerapawnref (`self.CameraPawnRef`))
  ;[1 1 1] Camera panning
  ;;[1 1 1] Pan Reset
  (:`Pressed`
    (`self.K2_SetActorRotation` _camerapawnref (`KismetMathLibrary.MakeRotator` (.roll (`self.K2_GetActorRotation` _camerapawnref))) false)))

(event `RemoveLocationDecal`
  (bind _targetlocationdecal (`self.TargetLocationDecal`))
  (`/Engine/EditorBlueprintResources/StandardMacros.IsValid` _targetlocationdecal
    (:`Is Valid`
      (`ActorComponent.K2_DestroyComponent` _targetlocationdecal))))

(event `Key|B`
  (params (Key :type "Key Structure"))
  (bind (_cursorlocationinworld_x _cursorlocationinworld_y) (`KismetMathLibrary.BreakVector` (`/Game/RTS_Test/Blueprints/Library/FuncLib.GetMousePosInWorld` self 10000.0)))
  (:`Pressed`
    (if true
      (`|SpawnActorFromClass` "/Game/RTS_Test/Blueprints/Units/GroundVehicles/RTS_GroundVehicleMaster.RTS_GroundVehicleMaster_C" (`KismetMathLibrary.MakeTransform` (`KismetMathLibrary.MakeVector` _cursorlocationinworld_x _cursorlocationinworld_y 100.0)) "DontSpawnIfColliding" "OverrideRootScale" null "NewEnumerator1" null))))

(event `Key|End`
  (params (Key :type "Key Structure"))
  (:`Pressed`
    (message `/Game/RTS_Test/Blueprints/Library/GameTime_IF.UpdateGameSpeed` (`self.GameStateRef`) 2.5e-05)))

(event `Key|V`
  (params (Key :type "Key Structure"))
  (bind (_cursorlocationinworld_x _cursorlocationinworld_y) (`KismetMathLibrary.BreakVector` (`/Game/RTS_Test/Blueprints/Library/FuncLib.GetMousePosInWorld` self 10000.0)))
  (:`Pressed`
    (if true
      (`|SpawnActorFromClass` "/Game/RTS_Test/Blueprints/Units/RTS_GroundUnitMaster.RTS_GroundUnitMaster_C" (`KismetMathLibrary.MakeTransform` (`KismetMathLibrary.MakeVector` _cursorlocationinworld_x _cursorlocationinworld_y 100.0)) "DontSpawnIfColliding" "OverrideRootScale" null null))))

(event `InputAction|PrimaryAction`
  (params (Key :type "Key Structure"))
  (:`Pressed`
    (if (`self.IsBuildingModeActive`)
      (if (not (`/Game/RTS_Test/Blueprints/Buildings/RTS_PreviewBuilding_BP.CheckOverlap` (`self.ConstructionPreviewRef`)))
        (bind _constructionstruct (`/Game/RTS_Test/Blueprints/Buildings/RTS_PreviewBuilding_BP.SetConstructionStructure` (`self.ConstructionPreviewRef`)))
        (`/Game/RTS_Test/Blueprints/Buildings/RTS_ConstructionManager_BP.StartConstruction` (`self.ConstructionManagerRef`) _constructionstruct)
        (`/Game/RTS_Test/Blueprints/Buildings/RTS_PreviewBuilding_BP.DestroyPreview` (`self.ConstructionPreviewRef`)))
      (else
        (message `/Game/RTS_Test/Blueprints/Library/MarqueeSelection_IF.OnInputStart` (`self.MarqueeHudRef`))
        (set `self.HoldingTime` 0.0)
        (set `self.IsHoldingInput` true))))
  (:`Released`
    (if (not (`self.IsBuildingModeActive`))
      (message `/Game/RTS_Test/Blueprints/Library/MarqueeSelection_IF.OnInputRelease` (`self.MarqueeHudRef`) (`self.HoldingTime`))
      (set `self.IsHoldingInput` false))))

(fn `GetUnitHud`
  (bind (_bblockinghit _binitialoverlap _time _distance _location _impactpoint _normal _impactnormal _physmat _hitactor) (`GameplayStatics.BreakHitResult` (`self.GetHitResultUnderCursorForObjects` (`self.SelectableObjectsEnum`))))
  (if (!= _hitactor null)
    (`self.DisplayUnitHud` _hitactor)))

(fn `SetBuildingModeActive`
  (params (IsActive :type Boolean))
  (set `self.IsBuildingModeActive` IsActive)
  (return))

(fn `SetHudVisibility`
  (params (MainGameHud :type "ESlateVisibility Enum" :default "Visible"))
  (`Widget.SetVisibility` (`self.MainGameHudRef`) MainGameHud))

(fn `SetSelectedUnits`
  (params (SelectedUnits :type "Array of /Game/RTS_Test/Blueprints/Units/RTS_GroundUnitMaster Object Reference") (SelectedVehicles :type "Array of /Game/RTS_Test/Blueprints/Units/GroundVehicles/RTS_GroundVehicleMaster Object Reference"))
  (set `self.SelectedUnits` SelectedUnits)
  (set `self.SelectedGroundVehicles` SelectedVehicles)
  (if (or (>= (`KismetArrayLibrary.Array_Length` (`self.SelectedUnits`)) 1) (>= (`KismetArrayLibrary.Array_Length` (`self.SelectedGroundVehicles`)) 1))
    (set `self.IsUnitSelected` true)))

(fn `UserConstructionScript`)
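; RTS player controller that drives the CameraPawn_BP camera with movement, edge scrolling, zoom and rotation.
; Caches the pawn on BeginPlay, then feeds key axes and screen-edge mouse checks into CameraMovement, a swept, yaw-relative move at fixed height, scaled by a boost modifier.
; Zoom adjusts spring arm length within limits and resets to its starting value.
; Holding Pan blocks movement and opens gates routing mouse axes to yaw and clamped pitch, with a separate reset.
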(event `self.ReceiveBeginPlay`
  (`|ExecutionSequence`
    (:`then_0`
      (`self.RefrenceCast`) ; Should always be first
    )
    (:`then_1`
      (set `self.StartZoom` (`SpringArmComponent.TargetArmLength` (`/Game/RTS_Test/Blueprints/GameSettings/CameraPawn_BP.SpringArm` (`self.CameraPawnRef`)))))))

(event `InputAxisKey|MouseX`
  (params (AxisValue :type "Float (single-precision)"))
  ;[1 1 1] Edge scroll movement
  (if (not (`self.DisableCameraMovement`))
    (bind (_deltaspeedx _deltaspeedy) (`self.EdgeScroll` :!label _label))
    (`self.CameraMovement` _deltaspeedx _deltaspeedy)))

(event `InputAxis|ZoomIn`
  (params (AxisValue :type "Float (single-precision)"))
  (bind _springarm (`/Game/RTS_Test/Blueprints/GameSettings/CameraPawn_BP.SpringArm` (`self.CameraPawnRef`)))
  ;[1 1 1] Camera Zoom
  ;;[1 1 1] Zoom in and out
  (set `SpringArmComponent.TargetArmLength` (`KismetMathLibrary.FClamp` (+ (`SpringArmComponent.TargetArmLength` _springarm) (* AxisValue (`self.ZoomSpeed`))) (`self.MinZoomLimit`) (`self.MaxZoomLimit`)) _springarm))

(event `InputAxisKey|MouseY`
  (params (AxisValue :type "Float (single-precision)"))
  ;[1 1 1] Edge scroll movement
  (if (not (`self.DisableCameraMovement`))
    (goto _label :!via `MouseY`)))

(event `InputAction|ZoomReset`
  (params (Key :type "Key Structure"))
  ;[1 1 1] Camera Zoom
  ;;[1 1 1] Zoom Reset
  (:`Pressed`
    (set `SpringArmComponent.TargetArmLength` (`self.StartZoom`) (`/Game/RTS_Test/Blueprints/GameSettings/CameraPawn_BP.SpringArm` (`self.CameraPawnRef`)))))

(event `InputAxis|MoveForward`
  (params (AxisValue :type "Float (single-precision)"))
  ;[1 1 1] Camera Movement
  (if (not (`self.DisableCameraMovement`)) :!label _label_2
    (`self.CameraMovement` AxisValue (stale `InputAxis|MoveRight` AxisValue))))

(event `InputAxis|MoveRight`
  (params (AxisValue :type "Float (single-precision)"))
  ;[1 1 1] Camera Movement
  (goto _label_2))

(event `InputAction|ZoomIn`
  (params (Key :type "Key Structure"))
  ;[1 1 1] Camera Zoom
  ;;[1 1 1] Old
)

(event `InputAction|FastCamera`
  (params (Key :type "Key Structure"))
  ;[1 1 1] Set Camera Boost
  (:`Pressed`
    (set `self.MovementSpeedModifier` 2.0))
  (:`Released`
    (set `self.MovementSpeedModifier` 1.0)))

(event `InputAction|ZoomOut`
  (params (Key :type "Key Structure"))
  ;[1 1 1] Camera Zoom
  ;;[1 1 1] Old
)

(event `InputAction|Pan`
  (params (Key :type "Key Structure"))
  (bind _camerapawnref (`self.CameraPawnRef`))
  ;[1 1 1] Camera panning
  ;;[1 1 1] Camera turning
  (:`Pressed`
    (set `self.DisableCameraMovement` true)
    (goto _label_3 :!via `Open`))
  (:`Released`
    (set `self.DisableCameraMovement` false)
    (goto _label_3 :!via `Close`)))

(event `InputAxisKey|MouseX`
  (params (AxisValue :type "Float (single-precision)"))
  (bind _camerapawnref (`self.CameraPawnRef`))
  ;[1 1 1] Camera panning
  ;;[1 1 1] Camera turning
  (`/Engine/EditorBlueprintResources/StandardMacros.Gate` true :!label _label_3
    (:`Exit`
      (`self.K2_SetActorRotation` _camerapawnref (`KismetMathLibrary.MakeRotator` (.roll (`self.K2_GetActorRotation` _camerapawnref)) (.pitch (`self.K2_GetActorRotation` _camerapawnref)) (+ (.yaw (`self.K2_GetActorRotation` _camerapawnref)) (* AxisValue (`self.PanSpeed`)))) false))))

(event `InputAction|Pan`
  (params (Key :type "Key Structure"))
  (bind _camerapawnref (`self.CameraPawnRef`))
  ;[1 1 1] Camera panning
  ;;[1 1 1] Camera turning
  (:`Pressed`
    (goto _label_4 :!via `Open`))
  (:`Released`
    (goto _label_4 :!via `Close`)))

(event `InputAxisKey|MouseY`
  (params (AxisValue :type "Float (single-precision)"))
  (bind _camerapawnref (`self.CameraPawnRef`))
  ;[1 1 1] Camera panning
  ;;[1 1 1] Camera turning
  (`/Engine/EditorBlueprintResources/StandardMacros.Gate` true :!label _label_4
    (:`Exit`
      (`self.K2_SetActorRotation` _camerapawnref (`KismetMathLibrary.MakeRotator` (.roll (`self.K2_GetActorRotation` _camerapawnref)) (`KismetMathLibrary.FClamp` (+ (.pitch (`self.K2_GetActorRotation` _camerapawnref)) (* AxisValue (`self.PanSpeed`))) -25.0 50.0) (.yaw (`self.K2_GetActorRotation` _camerapawnref))) false))))

(event `InputAction|PanReset`
  (params (Key :type "Key Structure"))
  (bind _camerapawnref (`self.CameraPawnRef`))
  ;[1 1 1] Camera panning
  ;;[1 1 1] Pan Reset
  (:`Pressed`
    (`self.K2_SetActorRotation` _camerapawnref (`KismetMathLibrary.MakeRotator` (.roll (`self.K2_GetActorRotation` _camerapawnref))) false)))

(fn `UserConstructionScript`)
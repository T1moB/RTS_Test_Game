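; RTS spawn volume that scatters resource actors at random points within its bounds, at BeginPlay, on a looping timer, or both.
; SpawnResource box-traces each random point and spawns only on Landscape hits, counting successes.
; Timed batches skip while paused or once the total cap is reached.
; The interval derives from game state speed, a custom value or their product; Tick recalculates it without restarting the timer.
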(event `self.ReceiveBeginPlay`
  (`|ExecutionSequence`
    (:`then_0`
      (`self.RefrenceCast`))
    (:`then_1`
      (add `/Game/RTS_Test/Blueprints/GameSettings/RTS_GameStateBase_BP.GameSpeedControl` (`self.GameStateRef`) (`|CreateDelegate` :!event `GetGameSpeed`))
      (bind _gamespeed (`/Game/RTS_Test/Blueprints/GameSettings/RTS_GameStateBase_BP.GetGameSpeed` (`self.GameStateRef`)))
      (set `self.GameSpeed` _gamespeed)
      (`self.SetRespawnTimer`))
    (:`then_2`
      (if (`self.IsSpawnedOnBeginPlay`)
        (`self.SpawnResource` (`self.ResourceRef`) (`self.NumOfResoucesSpawn`)))
      (if (`self.IsSpawnOnTimer`)
        (`KismetSystemLibrary.K2_SetTimerDelegate` (`|CreateDelegate` :!event `SpawnResourcerTimer`) (`self.ResourceRespawnTime`) true)))))

(event `GetGameSpeed`
  (params (GameSpeed :type "Float (double-precision)"))
  (set `self.GameSpeed` GameSpeed))

(event `self.ReceiveTick`
  (params (DeltaSeconds :type "Float (single-precision)"))
  (`self.SetRespawnTimer`))

(event `SpawnResourcerTimer`
  (if (`/Game/RTS_Test/Blueprints/Widgets/MainGameUI_HUD.IsPaused` (`/Game/RTS_Test/Blueprints/GameSettings/RTS_PlayerController_BP.MainGameHudRef` (`self.PlayerControllerRef`)))
    _
    (elif (< (`self.TotalNumberSpawned`) (`self.MaxResourcesSpawned`))
      (`self.SpawnResource` (`self.ResourceRef`) (`self.NumOfResoucesSpawn`)))))

(fn `SetRespawnTimer`
  (returns (RespawnTime :type "Float (double-precision)"))
  (switch `/Game/RTS_Test/Blueprints/Enums/RespawnTimer_ENUM` (`self.TimeSetting`)
    (:`NewEnumerator1`
      (set `self.ResourceRespawnTime` 0.0))
    (:`NewEnumerator2`
      (set `self.ResourceRespawnTime` (`self.GameSpeed`)))
    (:`NewEnumerator3`
      (set `self.ResourceRespawnTime` (`self.UserRespawnTimer`)))
    (:`NewEnumerator4`
      (set `self.ResourceRespawnTime` (* (`self.GameSpeed`) (`self.UserRespawnTimer`)))))
  (return (`self.ResourceRespawnTime`)))

(fn `SpawnResource`
  (params (Recourse :type "/Game/RTS_Test/Blueprints/Resources/ResourceMaster_BP Class Reference") (SpawnAmount :type Integer))
  (locals (ResourceRefLocal :type "/Game/RTS_Test/Blueprints/Resources/ResourceMaster_BP Class Reference") (SpawnAmountLocal :type Integer))
  (bind (_origin _boxextent) (`self.GetActorBounds` false))
  (bind _x (.x _boxextent))
  (bind _y (.y _boxextent))
  (bind _returnvalue (+ _origin (`KismetMathLibrary.MakeVector` (`KismetMathLibrary.RandomFloatInRange` (- _x (* _x 2.0)) _x) (`KismetMathLibrary.RandomFloatInRange` (- _y (* _y 2.0)) _y) (.z _origin))))
  (set `local.ResourceRefLocal` Recourse)
  (set `local.SpawnAmountLocal` SpawnAmount)
  (for _ (range (`local.SpawnAmountLocal`))
    (bind _outhit (`KismetSystemLibrary.BoxTraceSingle` (+ _returnvalue (0.0 0.0 100.0)) (0.0 0.0 0.0) (- _returnvalue (0.0 0.0 100.0)) (struct) "TraceTypeQuery1"))
    (bind (_bblockinghit _binitialoverlap _time _distance _location _impactpoint _normal _impactnormal _physmat _hitactor) (`GameplayStatics.BreakHitResult` _outhit))
    (if (== (`GameplayStatics.GetObjectClass` _hitactor) "/Script/Landscape.Landscape")
      (`|SpawnActorFromClass` (`local.ResourceRefLocal`) (`KismetMathLibrary.Conv_VectorToTransform` _location) "Undefined" "OverrideRootScale" null null)
      (`/Engine/EditorBlueprintResources/StandardMacros.IncrementInt` (`self.TotalNumberSpawned`)))))

(fn `UserConstructionScript`)
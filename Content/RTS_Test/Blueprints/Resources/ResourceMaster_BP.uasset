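; Base Blueprint for RTS resource objects that sets their starting amount and mesh appearance in the Construction Script.
; The resource level, optionally random, selects a multiplier that scales the base amount into current resources.
; Optional flags randomize mesh scale independently per axis within min/max bounds and spin the mesh to a random world yaw.
; Randomization is unseeded, so each construction run rerolls the enabled values.
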(fn `UserConstructionScript`
  (bind _returnvalue (`KismetMathLibrary.RandomFloatInRange` (`self.MinMeshSize`) (`self.MaxMeshSize`)))
  (`|ExecutionSequence`
    (:`then_0`
      (if (`self.IsRandomLevel`)
        (bind _output_get (set `self.ResourceLevelEnumRef` (cast `/Game/RTS_Test/Blueprints/Enums/ResourceLevel_ENUM` (`KismetMathLibrary.Conv_IntToByte` (`KismetMathLibrary.RandomIntegerInRange` 1 6))))))
      (switch `/Game/RTS_Test/Blueprints/Enums/ResourceLevel_ENUM` _output_get
        (:`NewEnumerator1`
          (set `self.ResourceModifier` 1.0))
        (:`NewEnumerator2`
          (set `self.ResourceModifier` 1.2))
        (:`NewEnumerator3`
          (set `self.ResourceModifier` 1.4))
        (:`NewEnumerator4`
          (set `self.ResourceModifier` 1.6))
        (:`NewEnumerator5`
          (set `self.ResourceModifier` 1.8))
        (:`NewEnumerator6`
          (set `self.ResourceModifier` 2.0)))
      (set `self.CurrentResources` (* (`self.BaseResourceAmount`) (`self.ResourceModifier`))))
    (:`then_1`
      (if (`self.IsRandomSize`)
        (`SceneComponent.SetWorldScale3D` (`self.ResourceMesh`) (`KismetMathLibrary.MakeVector` _returnvalue _returnvalue _returnvalue))))
    (:`then_2`
      (if (`self.IsRandomRotated`)
        (`SceneComponent.K2_SetWorldRotation` (`self.ResourceMesh`) (`KismetMathLibrary.MakeRotator` 0.0 0.0 (`KismetMathLibrary.RandomFloatInRange` 0.0 360.0)) false false)))))
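; Base RTS ground unit that gives each unit a random identity: sex, body color, name, age, portrait and birthday.
; Features roll in the construction script for spawned-in units, otherwise at BeginPlay; spawned units take the current game date as birthday.
; BirthDayEvent compares the game state's date to the birthday to increment age.
; A player controller event opens the unit's info HUD when it is the hit actor.
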(event `self.ReceiveBeginPlay`
  (`|ExecutionSequence`
    (:`then_0`
      (`self.ReferenceCast`)
      (add `/Game/RTS_Test/Blueprints/GameSettings/RTS_PlayerController_BP.DisplayUnitHud` (`self.ControllerRef`) (`|CreateDelegate` :!event `DisplayUnitHud`)))
    (:`then_2`
      (if (not (`self.IsSpawnedIn`))
        (`self.SetUnitFeatures`)))
    (:`then_3`
      (`self.SetUnitBirthday`))))

(event `BirthDayEvent`
  (bind _gamestateref (`self.GameStateRef`))
  (if (and (== (`/Game/RTS_Test/Blueprints/GameSettings/RTS_GameStateBase_BP.Month` _gamestateref) (`self.BirthMonth`)) (== (`/Game/RTS_Test/Blueprints/GameSettings/RTS_GameStateBase_BP.Day` _gamestateref) (`self.BirthDay`)))
    (bind _result (`/Engine/EditorBlueprintResources/StandardMacros.IncrementInt` (`self.UnitAge`))
      (:`  `
        (set `self.UnitAge` _result)
        (`KismetSystemLibrary.PrintText` (`KismetTextLibrary.Conv_StringToText` (`KismetStringLibrary.Concat_StrStr` "It's " (`self.UnitName`) " Birthday!")))))))

(event `DisplayUnitHud`
  (params (HitActor :type "Actor Object Reference") (Bypass :type Boolean :default false))
  (bind _controllerref (`self.ControllerRef`))
  (if (and (== self HitActor) (or Bypass (not (`self.IsHidden`))))
    (`UserWidget.AddToViewport` (`self.UnitHudRef`) 1)
    (`WidgetBlueprintLibrary.SetInputMode_UIOnlyEx` _controllerref null)
    (`Widget.SetIsEnabled` (`/Game/RTS_Test/Blueprints/GameSettings/RTS_PlayerController_BP.GameTimeHudRef` _controllerref) true)))

(fn `GetRandomName`
  (params (Sex :type Integer))
  (returns (UnitName :type String))
  (if (== Sex 0)
    (bind _output_get (set `self.MaleName` (`self.SetMaleName`)))
    (bind _output_get_2 (set `self.SurName` (`self.SetSurName`)))
    (return (`KismetStringLibrary.Concat_StrStr` (`|GetEnumeratorNameAsString` _output_get) " " (`|GetEnumeratorNameAsString` _output_get_2)))
    (else
      (bind _output_get_3 (set `self.FemaleName` (`self.SetFemaleName`)))
      (bind _output_get_4 (set `self.SurName` (`self.SetSurName`)))
      (return (`KismetStringLibrary.Concat_StrStr` (`|GetEnumeratorNameAsString` _output_get_3) " " (`|GetEnumeratorNameAsString` _output_get_4))))))

(fn `SetUnitBirthday`
  (bind _gamestateref (`self.GameStateRef`))
  (if (`self.IsSpawnedIn`)
    (set `self.BirthYear` (- (`/Game/RTS_Test/Blueprints/GameSettings/RTS_GameStateBase_BP.Year` (`self.GameStateRef`)) (`self.UnitAge`)))
    (set `self.BirthMonth` (`/Game/RTS_Test/Blueprints/GameSettings/RTS_GameStateBase_BP.Month` _gamestateref))
    (set `self.BirthDay` (`/Game/RTS_Test/Blueprints/GameSettings/RTS_GameStateBase_BP.Day` _gamestateref))
    (else
      (set `self.BirthYear` (- (`/Game/RTS_Test/Blueprints/GameSettings/RTS_GameStateBase_BP.Year` (`self.GameStateRef`)) (`self.UnitAge`)))
      (set `self.BirthMonth` (`KismetMathLibrary.RandomIntegerInRange` 1 12))
      (set `self.BirthDay` (`KismetMathLibrary.Clamp` (`KismetMathLibrary.RandomIntegerInRange` 1 31) 0 (`KismetMathLibrary.DaysInMonth` (`self.BirthYear`) (`self.BirthMonth`)))))))

(fn `SetUnitFeatures`
  (locals (MeshMatInstanceLocal :type "MaterialInstanceDynamic Object Reference"))
  (bind _meshmatinstancelocal (`local.MeshMatInstanceLocal`))
  (bind _returnvalue (`PrimitiveComponent.CreateDynamicMaterialInstance` (`self.Mesh`) 0 null "None"))
  (set `local.MeshMatInstanceLocal` _returnvalue)
  (set `self.UnitSex` (`KismetMathLibrary.RandomIntegerInRange` 0 1))
  (if (== (`self.UnitSex`) 0)
    (`MaterialInstanceDynamic.SetVectorParameterValue` _meshmatinstancelocal "BodyColor" (struct :`B` 1.0 :`A` 1.0))
    (bind _unitname (`self.GetRandomName` (`self.UnitSex`)))
    (set `self.UnitName` _unitname)
    (set `self.UnitAge` (`KismetMathLibrary.RandomIntegerInRange` 18 70))
    (set `self.UnitImage` (`self.MaleImage`))
    (else
      (`MaterialInstanceDynamic.SetVectorParameterValue` _meshmatinstancelocal "BodyColor" (struct :`R` 0.5 :`B` 0.5 :`A` 1.0))
      (bind _unitname_2 (`self.GetRandomName` (`self.UnitSex`)))
      (set `self.UnitName` _unitname_2)
      (set `self.UnitAge` (`KismetMathLibrary.RandomIntegerInRange` 18 70))
      (set `self.UnitImage` (`self.FemaleImage`))))
  (set `self.UnitProfile` (make `/Game/RTS_Test/Blueprints/Structures/RTS_UnitProfile_Struct` (`self.UnitName`) (`self.UnitSex`) (`self.UnitAge`) (`self.UnitImage`))))

(fn `UserConstructionScript`
  (if (`self.IsSpawnedIn`)
    (`self.SetUnitFeatures`)))
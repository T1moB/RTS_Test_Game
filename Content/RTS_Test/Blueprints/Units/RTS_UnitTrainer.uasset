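; RTS_UnitTrainer is a Blueprint that defines the resource cost of training units in the RTS test project.
; Its SetUnitCost function switches on unit type (Infantry, Engineer, Harvester or Support) and returns fixed wood and ore costs for each.
; The event graph and construction script are empty, so the file contains no spawning, queueing or resource-spending logic.
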(fn `SetUnitCost`
  (params (UnitType :type "/Game/RTS_Test/Blueprints/Enums/UnitTypes_ENUM Enum" :default "NewEnumerator0"))
  (returns (WoodCost :type "Float (double-precision)") (OreCost :type "Float (double-precision)"))
  (switch `/Game/RTS_Test/Blueprints/Enums/UnitTypes_ENUM` UnitType
    (:`NewEnumerator0`
      (set `self.WoodCost` 25.0)
      (set `self.OreCost` 75.0))
    (:`NewEnumerator1`
      (set `self.WoodCost` 50.0)
      (set `self.OreCost` 50.0))
    (:`NewEnumerator2`
      (set `self.WoodCost` 25.0)
      (set `self.OreCost` 25.0))
    (:`NewEnumerator3`
      (set `self.WoodCost` 75.0)
      (set `self.OreCost` 25.0)))
  (return (`self.WoodCost`) (`self.OreCost`)))

(fn `UserConstructionScript`)
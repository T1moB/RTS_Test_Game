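; RTS harvester unit that gathers wood or ore from a target resource and deposits it into the controller's stockpiles, capped at their maximums.
; A looping timer runs StartHarvesting, accumulating yield from game-speed-scaled time until inventory fills.
; It then depletes the resource, destroying it when empty, and AI-moves to the nearest resource building, or a random X offset if none exists.
; EarlyHarvestEnd stops harvesting and applies the partial depletion.
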(event `self.ReceiveTick`
  (params (DeltaSeconds :type "Float (single-precision)"))
  (set `self.DeltaTime` DeltaSeconds)
  (`self.OrientateToCamera`))

(event `self.HarvestTrigger`
  (`/Engine/EditorBlueprintResources/StandardMacros.IsValid` (`self.TargetResource`)
    (:`Is Valid`
      (`KismetSystemLibrary.K2_SetTimer` null "StartHarvesting" 0.01 true))))

(event `self.TriggerHarvestEnd`
  (bind (_returnvalue_x _returnvalue_y _returnvalue_z) (`KismetMathLibrary.BreakVector` (`SceneComponent.K2_GetComponentLocation` (`self.CapsuleComponent`))))
  (bind _currentresource (`self.ReduceTargetResource` (`self.TargetResource`)))
  (`self.DestroyTargetResource` _currentresource)
  (`self.SetTargetedResource` null)
  (set `self.TimeHarvesting` 0.0)
  (bind (_resourcebuildings _hasvalidtarget) (`/Game/RTS_Test/Blueprints/Library/FuncLib.GetResourceBuildings` (`self.ControllerRef`)))
  (if _hasvalidtarget
    (set `self.ResourceBuildings` _resourcebuildings)
    (bind _distancestobuildings (`self.GetDistanceToResourceBuildings`))
    (`self.SetTargetBuilding` (`self.GetNearestTarget` _distancestobuildings))
    (`AITask_MoveTo.AIMoveTo` (`AIBlueprintHelperLibrary.GetAIController` self) (`SceneComponent.K2_GetComponentLocation` (`/Game/RTS_Test/Blueprints/Buildings/RTS_BuildingMaster_BP.EntryPoint` (`self.TargetBuilding`))) null
      (:`OnMoveFinished`
        (`self.DepositResources`)
        (set `self.Harvested` 0.0)))
    (else
      (`AITask_MoveTo.AIMoveTo` (`AIBlueprintHelperLibrary.GetAIController` self) (`KismetMathLibrary.MakeVector` (+ (`KismetMathLibrary.RandomFloatInRange` 250.0 1000.0) _returnvalue_x) _returnvalue_y _returnvalue_z) null))))

(event `self.EarlyHarvestEnd`
  (`KismetSystemLibrary.K2_SetTimer` null "StartHarvesting")
  (if (> (`/Game/RTS_Test/Blueprints/Resources/ResourceMaster_BP.CurrentResources` (`self.TargetResource`)) 0.0)
    (bind _currentresource (`self.ReduceTargetResource` (`self.TargetResource`)))
    (`self.DestroyTargetResource` _currentresource)
    (`self.SetTargetedResource` null)))

(fn `DepositResources`
  (bind _controllerref (`self.ControllerRef`))
  (bind _maxwoodresource (`/Game/RTS_Test/Blueprints/GameSettings/RTS_PlayerController_BP.MaxWoodResource` _controllerref))
  (bind _maxoreresource (`/Game/RTS_Test/Blueprints/GameSettings/RTS_PlayerController_BP.MaxOreResource` _controllerref))
  (bind _returnvalue (+ (`/Game/RTS_Test/Blueprints/GameSettings/RTS_PlayerController_BP.WoodResources` _controllerref) (`self.WoodHarvested`)))
  (bind _returnvalue_2 (+ (`/Game/RTS_Test/Blueprints/GameSettings/RTS_PlayerController_BP.OreResources` _controllerref) (`self.OreHarvested`)))
  (if (>= _maxwoodresource _returnvalue)
    (set `/Game/RTS_Test/Blueprints/GameSettings/RTS_PlayerController_BP.WoodResources` _returnvalue _controllerref)
    (else
      (set `/Game/RTS_Test/Blueprints/GameSettings/RTS_PlayerController_BP.WoodResources` _maxwoodresource _controllerref)))
  (set `self.WoodHarvested` 0.0)
  (if (>= _maxoreresource _returnvalue_2)
    (set `/Game/RTS_Test/Blueprints/GameSettings/RTS_PlayerController_BP.OreResources` _returnvalue_2 _controllerref)
    (else
      (set `/Game/RTS_Test/Blueprints/GameSettings/RTS_PlayerController_BP.OreResources` _maxoreresource _controllerref)))
  (set `self.OreHarvested` 0.0)
  (return))

(fn `DestroyTargetResource`
  (params (CurrentResource :type "Float (double-precision)"))
  (if (<= CurrentResource 0.0)
    (`self.K2_DestroyActor` (`self.TargetResource`)))
  (return))

(fn `GetDistanceToResourceBuildings`
  (returns (DistancesToBuildings :type "Array of Float (double-precision)"))
  (locals (DistancesToBuildingsLocal :type "Array of Float (double-precision)"))
  (for _array_element (`self.ResourceBuildings`)
    (`KismetArrayLibrary.Array_AddUnique` (`local.DistancesToBuildingsLocal`) (`self.GetDistanceTo` _array_element)))
  (return (`local.DistancesToBuildingsLocal`)))

(fn `GetNearestTarget`
  (params (BuildingDistances :type "Array of Float (double-precision) (by ref)"))
  (returns (NearestBuilding :type "/Game/RTS_Test/Blueprints/Buildings/RTS_BuildingMaster_BP Object Reference"))
  (return (`|GetArrayItem` (`self.ResourceBuildings`) (`KismetMathLibrary.MinOfFloatArray` BuildingDistances))))

(fn `ReduceTargetResource`
  (params (TargetResource :type "/Game/RTS_Test/Blueprints/Resources/ResourceMaster_BP Object Reference"))
  (returns (CurrentResource :type "Float (double-precision)"))
  (locals (ResourceLocal :type "/Game/RTS_Test/Blueprints/Resources/ResourceMaster_BP Object Reference"))
  (bind _resourcelocal (`local.ResourceLocal`))
  (bind _resourcelocal_2 (`local.ResourceLocal`))
  (set `local.ResourceLocal` TargetResource)
  (switch `/Game/RTS_Test/Blueprints/Enums/ResourceType_ENUM` (`self.TargetedResourceType`)
    (:`NewEnumerator1`
      (set `/Game/RTS_Test/Blueprints/Resources/ResourceMaster_BP.CurrentResources` (- (`/Game/RTS_Test/Blueprints/Resources/ResourceMaster_BP.CurrentResources` _resourcelocal_2) (`self.CurrentWoodHarvest`)) _resourcelocal_2)
      (set `self.CurrentWoodHarvest` 0.0))
    (:`NewEnumerator2`
      (set `/Game/RTS_Test/Blueprints/Resources/ResourceMaster_BP.CurrentResources` (- (`/Game/RTS_Test/Blueprints/Resources/ResourceMaster_BP.CurrentResources` _resourcelocal) (`self.CurrentOreHarvest`)) _resourcelocal)
      (set `self.CurrentOreHarvest` 0.0)))
  (return (`/Game/RTS_Test/Blueprints/Resources/ResourceMaster_BP.CurrentResources` (`local.ResourceLocal`))))

(fn `StartHarvesting`
  (bind _output_get (set `self.TargetedResourceType` (`/Game/RTS_Test/Blueprints/Resources/ResourceMaster_BP.ResourceType` (`self.TargetResource`))))
  (switch `/Game/RTS_Test/Blueprints/Enums/ResourceType_ENUM` _output_get
    (:`NewEnumerator1`
      (bind _output_get_2 (set `self.TimeHarvesting` (`/Game/RTS_Test/Blueprints/Library/FuncLib.SetGameTime` (`self.DeltaTime`) (`self.GameSpeed`) (`self.TimeHarvesting`))))
      (set `self.CurrentWoodHarvest` (/ (* _output_get_2 60.0) 100.0))
      (set `self.Harvested` (+ (`self.OreHarvested`) (`self.WoodHarvested`) (`self.CurrentWoodHarvest`)))
      (if (<= (`self.MaxInventory`) (`self.Harvested`))
        (`KismetSystemLibrary.K2_SetTimer` null "StartHarvesting")
        (set `self.WoodHarvested` (+ (`self.CurrentWoodHarvest`) (`self.WoodHarvested`)))
        (set `self.IsInventoryFull` true :!label _label)
        (`self.TriggerHarvestEnd`)))
    (:`NewEnumerator2`
      (bind _output_get_3 (set `self.TimeHarvesting` (`/Game/RTS_Test/Blueprints/Library/FuncLib.SetGameTime` (`self.DeltaTime`) (`self.GameSpeed`) (`self.TimeHarvesting`))))
      (set `self.CurrentOreHarvest` (/ (* _output_get_3 60.0) 100.0))
      (set `self.Harvested` (+ (`self.OreHarvested`) (`self.WoodHarvested`) (`self.CurrentOreHarvest`)))
      (if (<= (`self.MaxInventory`) (`self.Harvested`))
        (`KismetSystemLibrary.K2_SetTimer` null "StartHarvesting")
        (set `self.OreHarvested` (+ (`self.CurrentOreHarvest`) (`self.OreHarvested`)))
        (goto _label)))))

(fn `UserConstructionScript`
  (`parent.UserConstructionScript`))
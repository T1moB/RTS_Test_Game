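; RTS engineer unit that repairs a target vehicle or building, carrying a toolbox attached to a mesh socket.
; RepairDamage checks for damage, then starts a fast looping timer calling RepairVehicle or RepairBuilding.
; Each tick adds points scaled by game speed and updates bars, restoring vehicle health before armor.
; On completion, values snap to maximum, and the engineer clears its busy state and leaves the target.
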(event `self.ReceiveBeginPlay`
  (`parent.ReceiveBeginPlay`)
  (if (not (`self.IsSpawnedIn`))
    (set `self.UnitType` "NewEnumerator1")))

(event `self.RepairDamage`
  (if (or (`self.CheckTargetHealth`) (`self.CheckArmorDamage`))
    (`/Engine/EditorBlueprintResources/StandardMacros.IsValid` (`self.TargetVehicle`)
      (:`Is Valid`
        (`KismetSystemLibrary.K2_SetTimer` null "RepairVehicle" 0.01 true))
      (:`Is Not Valid`
        (`/Engine/EditorBlueprintResources/StandardMacros.IsValid` (`self.TargetBuilding`)
          (:`Is Valid`
            (`KismetSystemLibrary.K2_SetTimer` null "RepairBuilding" 0.01 true)))))
    (else
      (`self.SetIsBusy` false))))

(fn `CheckArmorDamage`
  (returns (ReturnValue :type Boolean))
  (bind _targetvehicle (`self.TargetVehicle`))
  (`/Engine/EditorBlueprintResources/StandardMacros.IsValid` _targetvehicle
    (:`Is Valid`
      (return (< (`/Game/RTS_Test/Blueprints/Units/GroundVehicles/RTS_GroundVehicleMaster.CurrentArmor` _targetvehicle) (`/Game/RTS_Test/Blueprints/Units/GroundVehicles/RTS_GroundVehicleMaster.MaxArmor` _targetvehicle))))))

(fn `CheckTargetHealth`
  (returns (IsNotFullHealth :type Boolean))
  (locals (VehicleDamgeLocal :type Boolean) (BuildingDamageLocal :type Boolean))
  (bind _targetvehicle (`self.TargetVehicle`))
  (bind _targetbuilding (`self.TargetBuilding`))
  (`/Engine/EditorBlueprintResources/StandardMacros.IsValid` _targetvehicle
    (:`Is Valid`
      (set `local.VehicleDamgeLocal` (< (`/Game/RTS_Test/Blueprints/Units/GroundVehicles/RTS_GroundVehicleMaster.CurrentHealth` _targetvehicle) (`/Game/RTS_Test/Blueprints/Units/GroundVehicles/RTS_GroundVehicleMaster.MaxHealth` _targetvehicle))))
    (:`Is Not Valid`
      _))
  (`/Engine/EditorBlueprintResources/StandardMacros.IsValid` _targetbuilding
    (:`Is Valid`
      (set `local.BuildingDamageLocal` (< (`/Game/RTS_Test/Blueprints/Buildings/RTS_BuildingMaster_BP.CurrentHealth` _targetbuilding) (`/Game/RTS_Test/Blueprints/Buildings/RTS_BuildingMaster_BP.MaxHealth` _targetbuilding))))
    (:`Is Not Valid`
      _))
  (return (or (`local.VehicleDamgeLocal`) (`local.BuildingDamageLocal`))))

(fn `RepairBuilding`
  (bind _targetbuilding (`self.TargetBuilding`))
  (bind _targetbuilding_2 (`self.TargetBuilding`))
  (bind _output_get (set `self.RepairTime` (`/Game/RTS_Test/Blueprints/Library/FuncLib.SetGameTime` (`self.DeltaTime`) (`self.GameSpeed`) (`self.RepairTime`))))
  (set `/Game/RTS_Test/Blueprints/Buildings/RTS_BuildingMaster_BP.CurrentHealth` (+ (/ (* _output_get 60.0) 100.0) (`/Game/RTS_Test/Blueprints/Buildings/RTS_BuildingMaster_BP.CurrentHealth` _targetbuilding_2)) _targetbuilding_2)
  (`/Game/RTS_Test/Blueprints/Buildings/RTS_BuildingMaster_BP.UpdateHealthBar` _targetbuilding_2)
  (set `self.RepairTime` 0.01)
  (if (not (`self.CheckTargetHealth`))
    (set `/Game/RTS_Test/Blueprints/Buildings/RTS_BuildingMaster_BP.CurrentHealth` (`/Game/RTS_Test/Blueprints/Buildings/RTS_BuildingMaster_BP.MaxHealth` _targetbuilding) _targetbuilding)
    (`KismetSystemLibrary.K2_SetTimer` null "RepairBuilding")
    (`self.SetIsBusy` false)
    (`/Game/RTS_Test/Blueprints/Buildings/RTS_BuildingMaster_BP.ReleaseSingleOccupant` (`self.TargetBuilding`) self)
    (set `self.TargetBuilding` null)))

(fn `RepairVehicle`
  (bind _targetvehicle (`self.TargetVehicle`))
  (bind _targetvehicle_2 (`self.TargetVehicle`))
  (bind _targetvehicle_3 (`self.TargetVehicle`))
  (bind _targetvehicle_4 (`self.TargetVehicle`))
  (set `/Game/RTS_Test/Blueprints/Units/GroundVehicles/RTS_GroundVehicleMaster.IsUnderRepair` true (`self.TargetVehicle`))
  (if (`self.CheckTargetHealth`)
    (bind _output_get (set `self.RepairTime` (`/Game/RTS_Test/Blueprints/Library/FuncLib.SetGameTime` (`self.DeltaTime`) (`self.GameSpeed`) (`self.RepairTime`))))
    (set `/Game/RTS_Test/Blueprints/Units/GroundVehicles/RTS_GroundVehicleMaster.CurrentHealth` (+ (/ (* _output_get 60.0) 100.0) (`/Game/RTS_Test/Blueprints/Units/GroundVehicles/RTS_GroundVehicleMaster.CurrentHealth` _targetvehicle_2)) _targetvehicle_2)
    (`/Game/RTS_Test/Blueprints/Units/GroundVehicles/RTS_GroundVehicleMaster.UpdateHealthBar` _targetvehicle_2)
    (set `self.RepairTime` 0.01)
    (elif (`self.CheckArmorDamage`)
      (bind _output_get_2 (set `self.RepairTime` (`/Game/RTS_Test/Blueprints/Library/FuncLib.SetGameTime` (`self.DeltaTime`) (`self.GameSpeed`) (`self.RepairTime`))))
      (set `/Game/RTS_Test/Blueprints/Units/GroundVehicles/RTS_GroundVehicleMaster.CurrentArmor` (+ (/ (* _output_get_2 60.0) 100.0) (`/Game/RTS_Test/Blueprints/Units/GroundVehicles/RTS_GroundVehicleMaster.CurrentArmor` _targetvehicle)) _targetvehicle)
      (`/Game/RTS_Test/Blueprints/Units/GroundVehicles/RTS_GroundVehicleMaster.UpdateArmorBar` _targetvehicle)
      (set `self.RepairTime` 0.01)
      (else
        (set `self.RepairTime` 0.0)
        (set `/Game/RTS_Test/Blueprints/Units/GroundVehicles/RTS_GroundVehicleMaster.CurrentHealth` (`/Game/RTS_Test/Blueprints/Units/GroundVehicles/RTS_GroundVehicleMaster.MaxHealth` _targetvehicle_4) _targetvehicle_4)
        (set `/Game/RTS_Test/Blueprints/Units/GroundVehicles/RTS_GroundVehicleMaster.CurrentArmor` (`/Game/RTS_Test/Blueprints/Units/GroundVehicles/RTS_GroundVehicleMaster.MaxArmor` _targetvehicle_4) _targetvehicle_4)
        (`KismetSystemLibrary.K2_SetTimer` null "RepairVehicle")
        (`self.SetIsBusy` false)
        (set `/Game/RTS_Test/Blueprints/Units/GroundVehicles/RTS_GroundVehicleMaster.IsUnderRepair` false _targetvehicle_3)
        (`/Game/RTS_Test/Blueprints/Units/GroundVehicles/RTS_GroundVehicleMaster.RemoveSinglePassenger` _targetvehicle_3 self)
        (set `self.TargetVehicle` null)))))

(fn `UserConstructionScript`
  (`parent.UserConstructionScript`)
  (set `self.UnitType` "NewEnumerator1")
  (`SceneComponent.K2_AttachToComponent` (`self.ToolBox`) (`self.Mesh`) "ToolBox" "KeepRelative" "KeepRelative" "KeepRelative" true))